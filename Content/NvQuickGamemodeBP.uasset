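; Quick game mode Blueprint that brings up a Starburst session through a session selector.
; Game init adds an encode manager; Starburst init creates the selector, binds its deploy and exit callbacks, then starts session selection.
; The deploy callback deploys the satellite and a template from a stored path, while exit leads to an empty Starburst-initialized hook.
; BeginPlay is an empty placeholder for non-UI initialization, since UI created there gets overwritten.
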(event Custom|OnDeploy
  (Class|SBGSatelliteBP|DeploySatellite)
  (Class|SBGTemplateBP|DeployTemplate (Variables|Default|GetTemplatePath)))

(event EventOnStarburstInitialized
  (params (success :type Boolean))
  ;[1 1 1] You can setup your user interface here
)

(event EventOnInitGame
  (AddComponent|AddNvEncodeManagerBP))

(event EventOnInitStarburst
  (bind _returnvalue (AddComponent|AddSessionSelector))
  (EventDispatchers|BindEventtoOnDeploy _returnvalue (delegate Custom|OnDeploy))
  (EventDispatchers|BindEventtoOnExit _returnvalue (delegate EventOnStarburstInitialized))
  (Default|SelectSession _returnvalue))

(event EventBeginPlay
  ;[1 1 1] All initialization goes here except user interface (SBG would overwrite it)
)

(fn ConstructionScript)